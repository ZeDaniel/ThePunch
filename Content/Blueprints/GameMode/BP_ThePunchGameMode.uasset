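; Game mode Blueprint for ThePunch that spawns phase UI and restarts the level.
; Separate events each create and add a widget to the viewport for the micro game, the transition phase and the start of the transition phase.
; RestartGame reopens the current level by name, while BeginPlay and Tick do nothing.
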(event EventBeginPlay)

(event EventTick
  (params (DeltaSeconds :type Float%20%28single-precision%29)))

(event EventRestartGame
  (bind _returnvalue (Game|GetCurrentLevelName true))
  (Game|OpenLevel(byName) (Utilities|String|StringToName _returnvalue)))

(event EventRunStartTransitionPhaseUI
  (bind _returnvalue (UserInterface|CreateWidget "/Game/Blueprints/Widgets/BP_StartTransitionPhaseWidget.BP_StartTransitionPhaseWidget_C"))
  (UserInterface|Viewport|AddtoViewport _returnvalue 0))

(event EventRunTransitionPhaseUI
  (bind _returnvalue (UserInterface|CreateWidget "/Game/Blueprints/Widgets/BP_TransitionPhaseWidget.BP_TransitionPhaseWidget_C"))
  (UserInterface|Viewport|AddtoViewport _returnvalue 0))

(event EventRunMicroGameUI
  (bind _returnvalue (UserInterface|CreateWidget "/Game/Blueprints/Widgets/BP_MicroGameWidget.BP_MicroGameWidget_C"))
  (UserInterface|Viewport|AddtoViewport _returnvalue 0))

(fn ConstructionScript)